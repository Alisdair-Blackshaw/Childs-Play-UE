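; BPA_SpawnedLight is a short-lived point light actor that destroys itself after a timed intensity change.
; A setlightcolour event tints the light red for evil or blue otherwise, based on its IsEvil input.
; BeginPlay starts a timeline that multiplies the light's current intensity by its track value each update, so the change compounds, and destroys the actor on finish.
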(event Custom|set%20light%20colour
  (params (isEvil :type Boolean))
  (bind _pointlight (Variables|Default|GetPointLight))
  (if isEvil
    (Rendering|Components|Light|SetLightColor _pointlight "(R=1.000000,G=0.026817,B=0.000000,A=1.000000)" true)
    (else
      (Rendering|Components|Light|SetLightColor _pointlight "(R=0.000000,G=0.602177,B=1.000000,A=1.000000)" true))))

(event EventBeginPlay
  (bind _pointlight (Variables|Default|GetPointLight))
  (bind _newtrack_0 (Timeline|Timeline_0 PlayFromStart)
    (:Update
      (Rendering|Components|Light|SetIntensity _pointlight (* (Variables|/Script/Engine.LightComponentBase|GetIntensity _pointlight) _newtrack_0)))
    (:Finished
      (Actor|DestroyActor))))

(fn ConstructionScript)