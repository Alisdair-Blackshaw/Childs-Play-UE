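; BPA_LargeSpaceDoor is a door actor that lowers open or returns closed based on the actors overlapping its trigger Box.
; On BeginPlay it either forces the door open via JustForceOpen or records a baseline count of overlapping actors.
; Begin and end overlaps share one check comparing the current count to that baseline, using IsOpen to skip redundant moves.
; A MoveComponentTo node drives both directions, with debug prints reporting state.
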(event OnComponentBeginOverlap(Box)
  (params (OverlappedComponent :type Primitive%20Component%20Object%20Reference) (OtherActor :type Actor%20Object%20Reference) (OtherComp :type Primitive%20Component%20Object%20Reference) (OtherBodyIndex :type Integer) (bFromSweep :type Boolean) (SweepResult :type Hit%20Result%20Structure%20%28by%20ref%29))
  ;[0 0.6016 1] Open Door
  (if (not (Variables|Default|GetjustForceOpen))
    (Variables|Default|SetNumber%20of%20actors%20in%20box (Utilities|Array|Length (Collision|GetOverlappingActors (Variables|Default|GetBox) 0 :!class /Script/Engine.PrimitiveComponent)))
    (if (== (Variables|Default|GetNumber%20of%20actors%20in%20box) (Variables|Default|Getmin%20number%20of%20actors%20in%20box))
      (if (Variables|Default|GetisOpen)
        (Variables|Default|SetisOpen false)
        (goto _label_2 Return)
        (else
          (Development|PrintString "No need to change anything regarding this door" :!label _label)
          (Development|PrintString (Utilities|String|Append "Number of actors: " (Utilities|String|ToString(Integer) (Variables|Default|GetNumber%20of%20actors%20in%20box))))
          (Development|PrintString (Utilities|String|Append "closed number of actors: " (Utilities|String|ToString(Integer) (Variables|Default|Getmin%20number%20of%20actors%20in%20box))))))
      (elif (Variables|Default|GetisOpen)
        (goto _label)
        (else
          (Variables|Default|SetisOpen true)
          (Components|MoveComponentTo (Variables|Default|GetDoor) "0, 0,-180.000000" "0, 0, 0" false false 0.2 false :!label _label_2)
          (Development|PrintString (Utilities|String|Append "isOpen is set to: " (Utilities|String|ToString(Boolean) (Variables|Default|GetisOpen)))))))))

(event OnComponentEndOverlap(Box)
  (params (OverlappedComponent :type Primitive%20Component%20Object%20Reference) (OtherActor :type Actor%20Object%20Reference) (OtherComp :type Primitive%20Component%20Object%20Reference) (OtherBodyIndex :type Integer))
  ;[1 0.3047 0] Close Door
  (if (not (Variables|Default|GetjustForceOpen))
    (Variables|Default|SetNumber%20of%20actors%20in%20box (Utilities|Array|Length (Collision|GetOverlappingActors (Variables|Default|GetBox) 0 :!class /Script/Engine.PrimitiveComponent)))
    (if (== (Variables|Default|GetNumber%20of%20actors%20in%20box) (Variables|Default|Getmin%20number%20of%20actors%20in%20box))
      (if (Variables|Default|GetisOpen)
        (Variables|Default|SetisOpen false)
        (goto _label_2 Return)
        (else
          (Development|PrintString "No need to change anything regarding this door" :!label _label)
          (Development|PrintString (Utilities|String|Append "Number of actors: " (Utilities|String|ToString(Integer) (Variables|Default|GetNumber%20of%20actors%20in%20box))))
          (Development|PrintString (Utilities|String|Append "closed number of actors: " (Utilities|String|ToString(Integer) (Variables|Default|Getmin%20number%20of%20actors%20in%20box))))))
      (elif (Variables|Default|GetisOpen)
        (goto _label)
        (else
          (Variables|Default|SetisOpen true)
          (Components|MoveComponentTo (Variables|Default|GetDoor) "0, 0,-180.000000" "0, 0, 0" false false 0.2 false :!label _label_2)
          (Development|PrintString (Utilities|String|Append "isOpen is set to: " (Utilities|String|ToString(Boolean) (Variables|Default|GetisOpen)))))))))

(event Custom|Door%20Actor%20Check
  (if (Variables|Default|GetjustForceOpen)
    (Components|MoveComponentTo (Variables|Default|GetDoor) "0, 0,-180.000000" "0, 0, 0" false false 0.2 false)
    (else
      (Utilities|FlowControl|DoOnce false
        (:Completed
          (bind _result (Math|Integer|IncrementInt (Utilities|Array|Length (Collision|GetOverlappingActors (Variables|Default|GetBox) 0 :!class /Script/Engine.PrimitiveComponent)))
            (:%20%20
              (bind _result_2 (Math|Integer|DecrementInt _result)
                (:%20%20
                  (Variables|Default|Setmin%20number%20of%20actors%20in%20box _result_2))))))))))

(event EventBeginPlay
  (CallFunction|DoorActorCheck))

(event Collision|EventActorBeginOverlap
  (params (OtherActor :type Actor%20Object%20Reference)))

(event EventTick
  (params (DeltaSeconds :type Float%20%28single-precision%29)))

(fn ConstructionScript)