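; BPA_Bullet is a short-lived bullet actor whose point light fades out and determines its lifetime.
; A setlightcolour event tints the light red when IsEvil is true and blue otherwise.
; Tick lowers the light intensity at a constant rate scaled by delta time and destroys the actor once it reaches zero.
; The event graph contains no movement, collision or damage logic.
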(event Custom|set%20light%20colour
  (params (isEvil :type Boolean))
  (bind _pointlight (Variables|Default|GetPointLight))
  (if isEvil
    (Rendering|Components|Light|SetLightColor _pointlight "(R=1.000000,G=0.026817,B=0.000000,A=1.000000)" true)
    (else
      (Rendering|Components|Light|SetLightColor _pointlight "(R=0.000000,G=0.602177,B=1.000000,A=1.000000)" true))))

(event EventTick
  (params (DeltaSeconds :type Float%20%28single-precision%29))
  (bind _pointlight (Variables|Default|GetPointLight))
  (bind _intensity (Variables|/Script/Engine.LightComponentBase|GetIntensity _pointlight))
  (Rendering|Components|Light|SetIntensity _pointlight (- _intensity (* DeltaSeconds 1e+03)))
  (if (<= _intensity 0.0)
    (Actor|DestroyActor)))

(fn ConstructionScript)