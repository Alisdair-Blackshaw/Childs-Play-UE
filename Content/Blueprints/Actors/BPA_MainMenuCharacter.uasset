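; BPA_MainMenuCharacter is a main menu character actor intended to display a player's selected cosmetic.
; BeginPlay adds five skeletal mesh components at runtime and stores them in an array.
; UpdateCosmeticonDisplay prints a debug "Hello" and sets the SkeletalMesh variable to the array entry at the given cosmetic index.
; It only reassigns that reference, with no visibility or mesh asset changes.
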(event Custom|Update%20Cosmetic%20on%20Display
  (params (Player%20Cosmetic%20Int :type Integer))
  (Development|PrintString "Hello")
  (Variables|Default|SetSkeletalMesh (Utilities|Array|Get(acopy) (Variables|Default|GetNewVar_0) Player%20Cosmetic%20Int)))

(event EventBeginPlay
  (bind _returnvalue (AddComponent|AddSkeletalMeshComponent false))
  (bind _returnvalue_2 (AddComponent|AddSkeletalMeshComponent false))
  (bind _returnvalue_3 (AddComponent|AddSkeletalMeshComponent false))
  (bind _returnvalue_4 (AddComponent|AddSkeletalMeshComponent false))
  (bind _returnvalue_5 (AddComponent|AddSkeletalMeshComponent false))
  (Variables|Default|SetNewVar_0 (Utilities|Array|MakeArray _returnvalue _returnvalue_2 _returnvalue_3 _returnvalue_4 _returnvalue_5)))

(event Collision|EventActorBeginOverlap
  (params (OtherActor :type Actor%20Object%20Reference)))

(event EventTick
  (params (DeltaSeconds :type Float%20%28single-precision%29)))

(fn ConstructionScript)